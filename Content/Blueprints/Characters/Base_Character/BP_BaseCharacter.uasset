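; BP_BaseCharacter is a base character Blueprint whose only active logic is toggling the inventory screen.
; The Inventory input alternates through a FlipFlop between creating a new UI_Inventory widget and removing the stored one.
; Opening focuses the widget in Game and UI input mode with the cursor shown on BP_MainPlayerController; closing restores game-only input and hides the cursor.
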(event EventBeginPlay)

(event Collision|EventActorBeginOverlap
  (params (OtherActor :type Actor%20Object%20Reference)))

(event EventTick
  (params (DeltaSeconds :type Float%20%28single-precision%29)))

(event Input|ActionEvents|InputActionInventory
  (params (Key :type Key%20Structure))
  (bind _returnvalue (Game|GetPlayerController 0))
  (bind _asbp_main_player_controller (Utilities|Casting|CastToBP_MainPlayerController _returnvalue))
  (:Pressed
    (Utilities|FlowControl|FlipFlop
      (:A
        (bind _returnvalue_2 (UserInterface|CreateWidget "/Game/UI/Inventory/UI_Inventory.UI_Inventory_C" 0 0))
        (bind _output_get (Variables|Default|SetInventory%20UI%20Ref _returnvalue_2))
        (UserInterface|Viewport|AddtoViewport _output_get 0)
        (Input|SetInputModeGameandUI _asbp_main_player_controller _output_get "DoNotLock" false)
        (Variables|/Script/Engine.PlayerController|SetbShowMouseCursor _asbp_main_player_controller true))
      (:B
        (Utilities|IsValid (Variables|Default|GetInventory%20UI%20Ref)
          (:Is%20Valid
            (Widget|RemovefromParent (Variables|Default|GetInventory%20UI%20Ref))
            (Input|SetInputModeGameOnly _returnvalue)
            (Variables|/Script/Engine.PlayerController|SetbShowMouseCursor _returnvalue false)))))))

(fn ConstructionScript)