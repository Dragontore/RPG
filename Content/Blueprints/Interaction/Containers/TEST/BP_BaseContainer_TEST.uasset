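; BP_BaseContainer_TEST is a test interactable container whose lid opens on interaction and closes itself after a delay.
; Interact runs only on the authority, where the OpenLid timeline rotates TopMeshComp on roll, scaled by OpenAngle.
; Every timeline update calls CloseLid, which waits five seconds on a Delay, then reverses the timeline.
; BeginPlay and the construction script add no logic of their own.
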(event Custom|Close%20Lid
  (Utilities|FlowControl|Delay 5.0)
  (bind _open (Timeline|Open%20Lid Reverse)
    (:Update
      (Transformation|SetRelativeRotation (Variables|Default|GetTopMeshComp) (Math|Rotator|MakeRotator (* _open (Variables|Default|GetOpen%20Angle)) 0.0 0.0) false false)
      (CallFunction|CloseLid))))

(event EventBeginPlay
  (|CallParentFunction) ; This node is disabled and will not be called.\nDrag off pins to build functionality.
)

(event EventInteract
  (params (Player :type Base%20Character%20Object%20Reference))
  (Networking|SwitchHasAuthority
    (:Authority
      (bind _open (Timeline|Open%20Lid Play)
        (:Update
          (Transformation|SetRelativeRotation (Variables|Default|GetTopMeshComp) (Math|Rotator|MakeRotator (* _open (Variables|Default|GetOpen%20Angle)) 0.0 0.0) false false)
          (CallFunction|CloseLid))))))

(fn ConstructionScript
  (|CallParentFunction))