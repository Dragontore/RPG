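; BP_JudgeMent_Door is an interactable double door that swings open and closes itself automatically.
; On authority only, Interact plays two timelines that scale per-door angles into relative yaw on PropMeshComp (left) and StaticMesh (right).
; CloseDoor fires on every left-timeline update, relying on Delay ignoring calls while pending, and reverses both timelines after five seconds.
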(event Custom|Close%20Door
  (Utilities|FlowControl|Delay 5.0)
  (Utilities|FlowControl|Sequence
    (:then_0
      (bind _open_door (Timeline|Left%20Door Reverse)
        (:Update
          (Transformation|SetRelativeRotation (Variables|Default|GetPropMeshComp) (Math|Rotator|MakeRotator 0.0 0.0 (* _open_door (Variables|Default|GetLeft%20Door%20Angle))) false false)
          (CallFunction|CloseDoor))))
    (:then_1
      (bind _open_door_2 (Timeline|Right%20Door Reverse)
        (:Update
          (Transformation|SetRelativeRotation (Variables|Default|GetStaticMesh) (Math|Rotator|MakeRotator 0.0 0.0 (* _open_door_2 (Variables|Default|GetRight%20Door%20Angle))) false false))))))

(event EventBeginPlay
  (|CallParentFunction) ; This node is disabled and will not be called.\nDrag off pins to build functionality.
)

(event Collision|EventActorBeginOverlap
  (params (OtherActor :type Actor%20Object%20Reference))
  (|CallParentFunction OtherActor) ; This node is disabled and will not be called.\nDrag off pins to build functionality.
)

(event EventTick
  (params (DeltaSeconds :type Float%20%28single-precision%29))
  (|CallParentFunction DeltaSeconds) ; This node is disabled and will not be called.\nDrag off pins to build functionality.
)

(event EventInteract
  (params (Player :type Base%20Character%20Object%20Reference))
  (Networking|SwitchHasAuthority
    (:Authority
      (Utilities|FlowControl|Sequence
        (:then_0
          (bind _open_door (Timeline|Left%20Door Play)
            (:Update
              (Transformation|SetRelativeRotation (Variables|Default|GetPropMeshComp) (Math|Rotator|MakeRotator 0.0 0.0 (* _open_door (Variables|Default|GetLeft%20Door%20Angle))) false false)
              (CallFunction|CloseDoor))))
        (:then_1
          (bind _open_door_2 (Timeline|Right%20Door Play)
            (:Update
              (Transformation|SetRelativeRotation (Variables|Default|GetStaticMesh) (Math|Rotator|MakeRotator 0.0 0.0 (* _open_door_2 (Variables|Default|GetRight%20Door%20Angle))) false false))))))))

(fn ConstructionScript
  (|CallParentFunction))